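; Sliding door actor that rises when the player enters its trigger box, unless it is locked or requires a key.
; The Opening timeline drives the mesh height, then input is disabled and the PushCharacter timeline walks the player forward.
; After a short delay the door reverses shut, with a DoOnce, reset on each trigger, blocking repeat pushes.
; Input is not re-enabled here.
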(event OnComponentBeginOverlap(Box)
  (params (OverlappedComponent :type Primitive%20Component%20Object%20Reference) (OtherActor :type Actor%20Object%20Reference) (OtherComp :type Primitive%20Component%20Object%20Reference) (OtherBodyIndex :type Integer) (bFromSweep :type Boolean) (SweepResult :type Hit%20Result%20Structure%20%28by%20ref%29))
  (bind _returnvalue (Game|GetPlayerCharacter 0))
  (if (== OtherActor (Game|GetPlayerCharacter 0))
    (if (and (not (Variables|Default|GetRequiresKey)) (not (Variables|Default|GetLocked)))
      (CallFunction|OpenDoor)
      (Utilities|FlowControl|DoOnce false) ; enters at Reset
    )))

(event Custom|CloseDoor
  (bind _returnvalue (Game|GetPlayerCharacter 0))
  (bind _doorposition (Timeline|Opening Reverse)
    (:Update
      (Transformation|SetRelativeLocation (Variables|Default|GetStaticMesh) (+ (* "0, 0,310.000000" _doorposition) (Math|Vector|MakeVector 0.0 0.0 1.5e+02)) false false))
    (:Finished
      (Utilities|FlowControl|DoOnce false
        (:Completed
          (Input|DisableInput (Game|GetPlayerCharacter 0) (Game|GetPlayerController 0))
          (Timeline|PushCharacter PlayFromStart
            (:Update
              (Pawn|Input|AddMovementInput _returnvalue (Transformation|GetActorForwardVector _returnvalue) 1.0 false))
            (:Finished
              (Utilities|FlowControl|Delay 2.0)
              (CallFunction|CloseDoor))))))))

(event Custom|OpenDoor
  (bind _returnvalue (Game|GetPlayerCharacter 0))
  (bind _doorposition (Timeline|Opening PlayFromStart)
    (:Update
      (Transformation|SetRelativeLocation (Variables|Default|GetStaticMesh) (+ (* "0, 0,310.000000" _doorposition) (Math|Vector|MakeVector 0.0 0.0 1.5e+02)) false false))
    (:Finished
      (Utilities|FlowControl|DoOnce false
        (:Completed
          (Input|DisableInput (Game|GetPlayerCharacter 0) (Game|GetPlayerController 0))
          (Timeline|PushCharacter PlayFromStart
            (:Update
              (Pawn|Input|AddMovementInput _returnvalue (Transformation|GetActorForwardVector _returnvalue) 1.0 false))
            (:Finished
              (Utilities|FlowControl|Delay 2.0)
              (CallFunction|CloseDoor))))))))

(fn ConstructionScript)